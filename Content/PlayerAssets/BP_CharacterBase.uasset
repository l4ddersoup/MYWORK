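; Base character Blueprint that equips a weapon and supplies weapon-specific animations.
; On BeginPlay it calls AcquireNewWeapon, which spawns BP_WeaponBase with itself as owner and instigator, then attaches it to the mesh at the socket named in the weapon's class defaults.
; GetActiveWeaponAnims returns idle and walk animations from CurrentActiveWeapon, though the shown graphs never assign that variable.
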(event Custom|AcquireNewWeapon
  (params (WeaponClass :type BP%20Weapon%20Base%20Class%20Reference))
  (bind _equipsocketname (Utilities|GetClassDefaults WeaponClass))
  (bind _self self)
  (bind _returnvalue (Game|SpawnActorfromClass WeaponClass (Transformation|GetSocketTransform (Variables|Character|GetMesh) _equipsocketname "RTS_World") "Undefined" "MultiplyWithRoot" _self _self))
  (Transformation|AttachComponentToComponent _returnvalue (Variables|Character|GetMesh) _equipsocketname "KeepRelative" "KeepRelative" "KeepRelative" true))

(event Collision|EventActorBeginOverlap
  (params (OtherActor :type Actor%20Object%20Reference)))

(event EventTick
  (params (DeltaSeconds :type Float%20%28single-precision%29)))

(event EventBeginPlay
  (CallFunction|AcquireNewWeapon "/Game/Blueprints/Weapons/BP_WeaponBase.BP_WeaponBase_C"))

(fn ConstructionScript)

(fn GetActiveWeaponAnims
  (bind _currentactiveweapon (Variables|Default|GetCurrentActiveWeapon))
  (return (Variables|/Game/Blueprints/Weapons/BP_WeaponBase.BP_WeaponBase_C|GetIdleAnim _currentactiveweapon) (Variables|/Game/Blueprints/Weapons/BP_WeaponBase.BP_WeaponBase_C|GetWalkAnim _currentactiveweapon)))